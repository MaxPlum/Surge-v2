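; BP_Rotator is a spline path actor that, while overlapped, steers the player's view and position along its spline.
; The construction script builds a scaled cube spline mesh for each segment.
; Overlap events toggle a flag; while it is set, Tick sets control rotation 180 degrees around the nearest tangent.
; Tick also snaps the player capsule's X and Y to the spline, keeping Z, except at the endpoints.
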(event `self.ReceiveActorBeginOverlap`
  (params (OtherActor :type "Actor Object Reference"))
  (set `self.Rotator Active` true))

(event `self.ReceiveActorEndOverlap`
  (params (OtherActor :type "Actor Object Reference"))
  (set `self.Rotator Active` false))

(event `self.ReceiveTick`
  (params (DeltaSeconds :type "Float (single-precision)"))
  (bind _spline (`self.Spline`))
  (bind _capsulecomponent (`Character.CapsuleComponent` (`GameplayStatics.GetPlayerCharacter` 0)))
  (bind _returnvalue (`SceneComponent.K2_GetComponentLocation` _capsulecomponent))
  (bind _returnvalue_2 (`SplineComponent.FindLocationClosestToWorldLocation` _spline _returnvalue "World"))
  (if (`self.Rotator Active`)
    (`Controller.SetControlRotation` (`GameplayStatics.GetPlayerController` 0) (`KismetMathLibrary.RotatorFromAxisAndAngle` (`SplineComponent.FindTangentClosestToWorldLocation` _spline _returnvalue "World") 180.0))
    (if (not (or (== _returnvalue_2 (`SplineComponent.GetLocationAtSplinePoint` _spline 0 "World")) (== _returnvalue_2 (`SplineComponent.GetLocationAtSplinePoint` _spline (- (`SplineComponent.GetNumberOfSplinePoints` _spline) 1) "World"))))
      (`SceneComponent.K2_SetWorldLocation` _capsulecomponent (`KismetMathLibrary.MakeVector` (.x _returnvalue_2) (.y _returnvalue_2) (.z _returnvalue)) false false))))

(fn `UserConstructionScript`
  (bind _current_spline_mesh (`self.Current Spline Mesh`))
  (bind (_location _tangent) (`SplineComponent.GetLocationAndTangentAtSplinePoint` (`self.Spline`) (`self.Next Loop Index`) "Local"))
  (bind (_location_2 _tangent_2) (`SplineComponent.GetLocationAndTangentAtSplinePoint` (`self.Spline`) (`self.Current Loop Index`) "Local"))
  (`|ExecutionSequence`
    (:`then_0`
      (set `self.Num Spline Points` (`SplineComponent.GetNumberOfSplinePoints` (`self.Spline`))))
    (:`then_1`
      (for _index (range (+ (- (`self.Num Spline Points`) 2) 1))
        (bind _output_get (set `self.Current Loop Index` _index))
        (set `self.Next Loop Index` (+ _output_get 1))
        (set `self.Start Location` _location_2)
        (set `self.Start Tangent` _tangent_2)
        (set `self.End Location` _location)
        (set `self.End Tangent` _tangent)
        (bind _returnvalue (`AddComponent|NODE_AddSplineMeshComponent-0`))
        (bind _output_get_2 (set `self.Current Spline Mesh` _returnvalue))
        (`StaticMeshComponent.SetStaticMesh` _output_get_2 "/Game/Geometry/Meshes/1M_Cube.1M_Cube")
        (`SplineMeshComponent.SetStartAndEnd` _current_spline_mesh (`self.Start Location`) (`self.Start Tangent`) (`self.End Location`) (`self.End Tangent`) true)
        (`SplineMeshComponent.SetStartScale` _current_spline_mesh (10.0 10.0) true)
        (`SplineMeshComponent.SetEndScale` _current_spline_mesh (10.0 10.0) true)
        (`KismetArrayLibrary.Array_AddUnique` (`self.Meshes`) _current_spline_mesh)))))